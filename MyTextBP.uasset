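; MyTextBP is a countdown text actor that adds an explosion effect when its countdown finishes.
; It overrides the parent's CountdownHasFinished event, calls the parent version, then spawns the P_Explosion emitter at the CountdownText component's world location.
; The construction script sets the initial placeholder text; the countdown logic itself is not in this Blueprint, and a leftover SetText node is unconnected.
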(event `self.ReceiveBeginPlay`)

(event `self.ReceiveActorBeginOverlap`
  (params (OtherActor :type "Actor Object Reference")))

(event `self.ReceiveTick`
  (params (DeltaSeconds :type "Float (single-precision)")))

(event `self.CountdownHasFinished`
  ;[1 1 1] 重写父类方法，里面调用父类方法
  (`parent.CountdownHasFinished`)
  (`GameplayStatics.SpawnEmitterAtLocation` "/Game/StarterContent/Particles/P_Explosion.P_Explosion" (`SceneComponent.K2_GetComponentLocation` (`self.CountdownText`))))

(fn `UserConstructionScript`
  (`TextRenderComponent.K2_SetText` (`self.CountdownText`) (`KismetTextLibrary.Conv_StringToText` "init text")))